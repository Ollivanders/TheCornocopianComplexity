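; Gap is a cave layout actor that pushes itself horizontally until it no longer overlaps other Gap or Wall actors.
; Its construction script picks random X and Y step factors, and on begin overlap a while loop repeatedly teleports it along that direction, scaled by RoomAdjustmentRate.
; Setter functions supply that rate and resize the collision box.
; Unconnected leftovers hold alternative approaches, including moving away from Room_display actors and eight-way direction selection.
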(event Collision|EventActorBeginOverlap
  (params (OtherActor :type Actor%20Object%20Reference))
  (bind _room_adjustment_rate (Variables|Default|GetRoom%20Adjustment%20Rate))
  (while (or (> (Utilities|Array|Length (Collision|GetOverlappingActors "Gap_C" :!class /Script/Engine.Actor)) 0) (> (Utilities|Array|Length (Collision|GetOverlappingActors "/Game/Game/Blueprints/Caves/Wall.Wall_C" :!class /Script/Engine.Actor)) 0))
    (Transformation|SetActorLocation (+ (Transformation|GetActorLocation) (Math|Vector|MakeVector (* (Variables|Default|Getxchange) _room_adjustment_rate) (* (Variables|Default|Getychange) _room_adjustment_rate) 0.0)) false true)))

(fn ConstructionScript
  (Variables|Default|Setxchange (Math|Random|RandomFloatinRange -1.0 1.0))
  (Variables|Default|Setychange (Math|Random|RandomFloatinRange -1.0 1.0)))

(fn SetCollisionExtent
  (params (CollisionExtent :type Float%20%28single-precision%29))
  (Components|Box|SetBoxExtent (Variables|Default|GetBox) (Math|Vector|MakeVector CollisionExtent CollisionExtent 5e+01) true))

(fn SetRoomAdjustment
  (params (Room%20Adjustment%20Rate :type Float%20%28single-precision%29))
  (Variables|Default|SetRoom%20Adjustment%20Rate Room%20Adjustment%20Rate))