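; Cave wall actor that pushes itself clear of overlapping actors, apparently as a room-separation step in cave layout generation.
; The construction script picks a random XY drift, and on actor overlap a loop repeatedly moves the wall along it, scaled by RoomAdjustmentRate, until nothing overlaps.
; Setter functions expose that rate and the box collision extent.
; Alternative logic for pushing away from neighboring rooms and choosing compass directions is disconnected.
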(event OnComponentBeginOverlap(Box)
  (params (OverlappedComponent :type Primitive%20Component%20Object%20Reference) (OtherActor :type Actor%20Object%20Reference) (OtherComp :type Primitive%20Component%20Object%20Reference) (OtherBodyIndex :type Integer) (bFromSweep :type Boolean) (SweepResult :type Hit%20Result%20Structure%20%28by%20ref%29)))

(event Collision|EventActorBeginOverlap
  (params (OtherActor :type Actor%20Object%20Reference))
  (bind _room_adjustment_rate (Variables|Default|GetRoom%20Adjustment%20Rate))
  (while (> (Utilities|Array|Length (Collision|GetOverlappingActors 0 :!class /Script/Engine.Actor)) 0)
    (Transformation|SetActorLocation (+ (Transformation|GetActorLocation) (Math|Vector|MakeVector (* (Variables|Default|Getxchange) _room_adjustment_rate) (* (Variables|Default|Getychange) _room_adjustment_rate) 0.0)) true true)))

(event EventBeginPlay)

(fn ConstructionScript
  (Variables|Default|Setxchange (Math|Random|RandomFloatinRange -1.0 1.0))
  (Variables|Default|Setychange (Math|Random|RandomFloatinRange -1.0 1.0)))

(fn SetCollisionExtent
  (params (CollionExtent :type Float%20%28single-precision%29))
  (Components|Box|SetBoxExtent (Variables|Default|GetBox) (Math|Vector|MakeVector CollionExtent CollionExtent 5e+01) true))

(fn SetRoomAdjustment
  (params (Room%20Adjustment :type Float%20%28single-precision%29))
  (Variables|Default|SetRoom%20Adjustment%20Rate Room%20Adjustment))