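; LargeRoom_Filter is an actor with a box collision, apparently a large-room placeholder for spreading out overlapping rooms in a generated layout.
; Its construction script randomizes X and Y offsets from NetDirection, and SetCollisionExtent sizes the box's square footprint.
; The overlap-driven push-apart loops that would move it away from Room_display and LargeRoom_display actors are disconnected, as is an unfinished eight-way direction picker with all-zero offsets.
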(fn ConstructionScript
  (bind _netdirection (Variables|Default|GetNetDirection))
  (bind _netdirection_2 (Variables|Default|GetNetDirection))
  (Variables|Default|Setxchange (Math|Random|RandomFloatinRange (* _netdirection -1.0) _netdirection))
  (Variables|Default|Setychange (Math|Random|RandomFloatinRange _netdirection_2 (* (- _netdirection_2 -2.0) -1.0))))

(fn SetCollisionExtent
  (params (CollisionExtent :type Float%20%28single-precision%29))
  (Components|Box|SetBoxExtent (Variables|Default|GetBox) (Math|Vector|MakeVector CollisionExtent CollisionExtent 5e+01) true))