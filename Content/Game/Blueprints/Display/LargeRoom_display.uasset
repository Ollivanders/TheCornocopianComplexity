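; LargeRoom_display is a large-room placeholder actor that pushes itself apart from other room displays, apparently for a generated layout.
; The construction script picks random X and Y drift values from NetDirection.
; On overlap, a while loop teleports it along that drift, scaled by RoomAdjustmentRate, until no Room_display or LargeRoom_display overlaps remain.
; SetCollisionExtent sizes its square collision box; averaged-position repulsion and eight-way direction logic are left unconnected.
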(event Collision|EventActorBeginOverlap
  (params (OtherActor :type Actor%20Object%20Reference))
  (bind _room_adjustment_rate (Variables|Default|GetRoom%20Adjustment%20Rate))
  (while (or (> (Utilities|Array|Length (Collision|GetOverlappingActors "/Game/Game/Blueprints/Display/Room_display.Room_display_C" :!class /Script/Engine.Actor)) 0) (> (Utilities|Array|Length (Collision|GetOverlappingActors "LargeRoom_display_C" :!class /Script/Engine.Actor)) 0))
    (Transformation|SetActorLocation (+ (Transformation|GetActorLocation) (Math|Vector|MakeVector (* (Variables|Default|Getxchange) _room_adjustment_rate) (* (Variables|Default|Getychange) _room_adjustment_rate) 0.0)) false true)))

(fn ConstructionScript
  (bind _netdirection (Variables|Default|GetNetDirection))
  (bind _netdirection_2 (Variables|Default|GetNetDirection))
  (Variables|Default|Setxchange (Math|Random|RandomFloatinRange (* _netdirection -1.0) _netdirection))
  (Variables|Default|Setychange (Math|Random|RandomFloatinRange _netdirection_2 (* (- _netdirection_2 -2.0) -1.0))))

(fn SetCollisionExtent
  (params (CollisionExtent :type Float%20%28single-precision%29))
  (Components|Box|SetBoxExtent (Variables|Default|GetBox) (Math|Vector|MakeVector CollisionExtent CollisionExtent 5e+01) true))