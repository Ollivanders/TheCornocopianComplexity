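; Room display actor that pushes itself clear of overlapping Room_display and LargeRoom_display actors, apparently to spread out a room layout.
; The construction script picks random X/Y drift from NetDirection, which a begin-overlap loop scales by RoomAdjustmentRate and applies as swept teleports until overlaps end.
; SetCollisionExtent sizes the square box footprint.
; Disconnected graphs hold alternative average-position repulsion and eight-way direction logic.
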(event OnComponentBeginOverlap(Box)
  (params (OverlappedComponent :type Primitive%20Component%20Object%20Reference) (OtherActor :type Actor%20Object%20Reference) (OtherComp :type Primitive%20Component%20Object%20Reference) (OtherBodyIndex :type Integer) (bFromSweep :type Boolean) (SweepResult :type Hit%20Result%20Structure%20%28by%20ref%29)))

(event Collision|EventActorBeginOverlap
  (params (OtherActor :type Actor%20Object%20Reference))
  (bind _room_adjustment_rate (Variables|Default|GetRoom%20Adjustment%20Rate))
  (while (or (> (Utilities|Array|Length (Collision|GetOverlappingActors "Room_display_C" :!class /Script/Engine.Actor)) 0) (> (Utilities|Array|Length (Collision|GetOverlappingActors "/Game/Game/Blueprints/Display/LargeRoom_display.LargeRoom_display_C" :!class /Script/Engine.Actor)) 0))
    (Transformation|SetActorLocation (+ (Transformation|GetActorLocation) (Math|Vector|MakeVector (* (Variables|Default|Getxchange) _room_adjustment_rate) (* (Variables|Default|Getychange) _room_adjustment_rate) 0.0)) true true)))

(fn ConstructionScript
  (bind _net_direction (Variables|Default|GetNet%20Direction))
  (bind _net_direction_2 (Variables|Default|GetNet%20Direction))
  (bind _returnvalue (- _net_direction 2.0))
  (Variables|Default|Setxchange (Math|Random|RandomFloatinRange (* _net_direction_2 -1.0) _net_direction_2))
  (Variables|Default|Setychange (Math|Random|RandomFloatinRange _returnvalue (* _returnvalue -1.0))))

(fn SetCollisionExtent
  (params (CollionExtent :type Float%20%28single-precision%29))
  (Components|Box|SetBoxExtent (Variables|Default|GetBox) (Math|Vector|MakeVector CollionExtent CollionExtent 5e+01) true))