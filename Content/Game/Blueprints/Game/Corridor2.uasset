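; Corridor actor for what appears to be a procedural room layout, which shifts itself until it is clear of other corridors and main rooms.
; The construction script picks one of eight compass directions, with random skewed variants, as an X/Y step.
; On actor overlap, a while loop teleports it by that step until no Corridor or MainRoom overlaps remain.
; Side-component removal and averaged-position repulsion logic are disconnected and never run.
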(event OnComponentBeginOverlap(Box)
  (params (OverlappedComponent :type Primitive%20Component%20Object%20Reference) (OtherActor :type Actor%20Object%20Reference) (OtherComp :type Primitive%20Component%20Object%20Reference) (OtherBodyIndex :type Integer) (bFromSweep :type Boolean) (SweepResult :type Hit%20Result%20Structure%20%28by%20ref%29)))

(event Collision|EventActorBeginOverlap
  (params (OtherActor :type Actor%20Object%20Reference))
  (while (or (> (Utilities|Array|Length (Collision|GetOverlappingActors "/Game/Game/Blueprints/Game/Corridor.Corridor_C" :!class /Script/Engine.Actor)) 0) (> (Utilities|Array|Length (Collision|GetOverlappingActors "/Game/Game/Blueprints/Game/MainRoom.MainRoom_C" :!class /Script/Engine.Actor)) 0))
    (Transformation|SetActorLocation (+ (Transformation|GetActorLocation) (Math|Vector|MakeVector (* (Variables|Default|Getxchange) 1.0) (* (Variables|Default|Getychange) 1.0) 0.0)) false true)))

(fn ConstructionScript
  (bind _output_get (Variables|Default|SetDirection (Math|Random|RandomIntegerinRange 1 8)))
  (if (== _output_get 1)
    ;[1 1 1] N
    (Variables|Default|Setxchange 0)
    (Variables|Default|Setychange 1)
    (if (== (Math|Random|RandomIntegerinRange 0 1) 0)
      (Variables|Default|Setxchange 1)
      (Variables|Default|Setychange 2))
    (elif (== _output_get 2)
      ;[1 1 1] NE
      (Variables|Default|Setxchange 1)
      (Variables|Default|Setychange 1)
      (if (== (Math|Random|RandomIntegerinRange 0 1) 0)
        (Variables|Default|Setxchange 2)
        (Variables|Default|Setychange 1))
      (elif (== _output_get 3)
        ;[1 1 1] E
        (Variables|Default|Setxchange 1)
        (Variables|Default|Setychange 0)
        (if (== (Math|Random|RandomIntegerinRange 0 1) 0)
          (Variables|Default|Setxchange 2)
          (Variables|Default|Setychange -1))
        (elif (== _output_get 4)
          ;[1 1 1] SE
          (Variables|Default|Setxchange 1)
          (Variables|Default|Setychange -1)
          (if (== (Math|Random|RandomIntegerinRange 0 1) 0)
            (Variables|Default|Setxchange 1)
            (Variables|Default|Setychange -2))
          (elif (== _output_get 5)
            ;[1 1 1] S
            (Variables|Default|Setxchange 0)
            (Variables|Default|Setychange -1)
            (if (== (Math|Random|RandomIntegerinRange 0 1) 0)
              (Variables|Default|Setxchange -1)
              (Variables|Default|Setychange -2))
            (elif (== _output_get 6)
              ;[1 1 1] SW
              (Variables|Default|Setxchange -1)
              (Variables|Default|Setychange -1)
              (if (== (Math|Random|RandomIntegerinRange 0 1) 0)
                (Variables|Default|Setxchange -2)
                (Variables|Default|Setychange -1))
              (elif (== _output_get 7)
                ;[1 1 1] W
                (Variables|Default|Setxchange -1)
                (Variables|Default|Setychange 0)
                (if (== (Math|Random|RandomIntegerinRange 0 1) 0)
                  (Variables|Default|Setxchange -2)
                  (Variables|Default|Setychange 1))
                (elif (== _output_get 8)
                  ;[1 1 1] NW
                  (Variables|Default|Setxchange -1)
                  (Variables|Default|Setychange 1)
                  (if (== (Math|Random|RandomIntegerinRange 0 1) 0)
                    (Variables|Default|Setxchange -1)
                    (Variables|Default|Setychange 2)))))))))))