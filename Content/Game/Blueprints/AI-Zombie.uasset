(event OnSeePawn(PawnSensing)
  (params (Pawn :type Pawn%20Object%20Reference))
  (Variables|Default|SetInitalLocation (Transformation|GetActorLocation))
  (if (Variables|Default|GethasSeen)
    (Utilities|FlowControl|Delay 1.0)
    (bind _ascharacter (Utilities|Casting|CastToCharacter Pawn))
    (AI|AIMoveTo self "0, 0, 0" _ascharacter 5.0 false
      (:OnSuccess
        (Development|PrintString "You Lose" true true "(R=1.000000,G=0.000000,B=0.102115,A=1.000000)")
        (Utilities|FlowControl|Delay 1.0)
        (Game|QuitGame 0 "Quit" false)))
    (else
      (Variables|Default|SethasSeen true)
      (Utilities|FlowControl|Delay 1.0)
      (bind _ascharacter_2 (Utilities|Casting|CastToCharacter Pawn))
      (AI|AIMoveTo self "0, 0, 0" _ascharacter_2 5.0 false
        (:then
          (Utilities|FlowControl|Delay 1.0)
          (AI|SpawnAIFromClass "AI-Zombie_C" 0 (Variables|Default|GetInitalLocation) (Math|Rotator|MakeRotator 0.0 0.0 (Math|Random|RandomFloatinRange 0.0 3.6e+02)) false))
        (:OnSuccess
          (Game|QuitGame 0 "Quit" false))))))

(event EventBeginPlay
  (Variables|/Script/Engine.CharacterMovementComponent|SetMaxWalkSpeed (Variables|Character|GetCharacterMovement self) 4.5e+02))

(fn ConstructionScript)